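; NPC character that roams the navmesh, chases characters it sees, and dies from damage.
; Tick starts slow AIMoveTo walks to random reachable points, gated by InRange and Moving flags with pauses between moves.
; PawnSensing triggers a faster chase, and roaming resumes after a delay once that move ends.
; At zero health the mesh ragdolls, then the actor destroys itself and spawns a replacement at a fixed location.
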(event `self.PawnSensing.OnSeePawn`
  (params (Pawn :type "Pawn Object Reference"))
  ;[1 1 1] Run and attack player when they enter field of vision
  (set `self.InRange` true)
  (set `CharacterMovementComponent.MaxWalkSpeed` 450.0 (`self.CharacterMovement`))
  (bind _ascharacter (cast `Character` Pawn))
  (`|AIMoveTo` self (0.0 0.0 0.0) _ascharacter 5.0
    (:`OnSuccess`
      _)
    (:`OnFail`
      _))
  (`KismetSystemLibrary.Delay` 5.0)
  (set `self.InRange` false))

(event `self.ReceiveTick`
  (params (DeltaSeconds :type "Float (single-precision)"))
  ;[1 1 1] Random roaming
  (if (`self.InRange`)
    _
    (elif (not (`self.Moving`))
      (`|AIMoveTo` self (`NavigationSystem.GetRandomPointInNavigableRadius` (`SceneComponent.K2_GetComponentLocation` (`self.Mesh`)) 10000.0)
        (:`then`
          (set `self.Moving` true)
          (set `CharacterMovementComponent.MaxWalkSpeed` 200.0 (`self.CharacterMovement`)))
        (:`OnSuccess`
          (`KismetSystemLibrary.Delay` 1.5 :!label _label)
          (set `self.Moving` false))
        (:`OnFail`
          (goto _label))))))

(event `self.ReceiveAnyDamage`
  (params (Damage :type "Float (single-precision)") (DamageType :type "DamageType Object Reference") (InstigatedBy :type "Controller Object Reference") (DamageCauser :type "Actor Object Reference"))
  ;[1 1 1] AI health & ragdoll death
  (bind _output_get (set `self.Health` (- (`self.Health`) Damage)))
  (if (<= _output_get 0.0)
    (`PrimitiveComponent.SetSimulatePhysics` (`self.Mesh`) true)
    (`ActorComponent.K2_DestroyComponent` (`self.CapsuleComponent`))
    (`ActorComponent.K2_DestroyComponent` (`self.CollisionCapsule`))
    (`KismetSystemLibrary.Delay` 5.0)
    (`self.K2_DestroyActor`)
    ;[1 1 1] Respawn
    (`AIBlueprintHelperLibrary.SpawnAIFromClass` "NPCCharacter_C" null (-760.0 -1590.0 520.0) (struct) true)))

(fn `UserConstructionScript`)