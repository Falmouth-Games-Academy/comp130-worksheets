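; Enemy character that attacks the player at close range and hands its replacement to Enemy_BP_Spawner on death.
; Tick scales the health bar and checks player distance, triggering a DoOnce-gated attack that only flashes a light and text, dealing no damage.
; At zero health, Tick calls Death without a guard, shattering the destructible mesh.
; After a delay, Death has the spawner delist it and spawn another, then destroys itself.
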(event `self.ReceiveBeginPlay`
  ;[1 1 1] Initialise movement speed and set spawner for control
  (set `CharacterMovementComponent.MaxWalkSpeed` (`self.MaxWalkSpeed`) (`self.CharacterMovement`))
  (bind _outactors (`GameplayStatics.GetAllActorsOfClass` "/Game/Enemy_BP_Spawner.Enemy_BP_Spawner_C"))
  (set `self.Enemy_BP_Spawner` (`KismetArrayLibrary.Array_Get` _outactors))
  (set `self.Health` (`self.EnemyMaxHealth`)))

(event `self.ReceiveTick`
  (params (DeltaSeconds :type "Float (single-precision)"))
  ;[1 1 1] Size Health Bar
  (`SceneComponent.SetWorldScale3D` (`self.HealthBar`) (`KismetMathLibrary.MakeVector` 0.1 (/ (`self.Health`) (`self.EnemyMaxHealth`)) 0.1))
  ;[1 1 1] Check if enemy has died
  (if (<= (`self.Health`) 0.0)
    (`self.Event Death`)
    (elif (< (`self.GetDistanceTo` self (`GameplayStatics.GetPlayerPawn` 0)) (`self.AttackDistance`))
      (`/Engine/EditorBlueprintResources/StandardMacros.DoOnce` false :!label _label
        (:`Completed`
          (`self.Event AttackPlayer`))))))

(event `Event AttackPlayer`
  ;[1 1 1] Attacking
  ;;[1 1 1] Flashes Red and attacks with words
  (`LightComponent.SetLightColor` (`self.AttackLight`) (`self.AttackColour`) true)
  (`SceneComponent.SetVisibility` (`self.AttackText`) true false)
  (`KismetSystemLibrary.Delay` 0.5)
  ;;[1 1 1] Reset to passive
  (`LightComponent.SetLightColor` (`self.AttackLight`) (`self.PassiveColour`) true)
  (`SceneComponent.SetVisibility` (`self.AttackText`) false false)
  (`KismetSystemLibrary.Delay` 0.2)
  (goto _label :!via `Reset`))

(event `Event Death`
  ;[1 1 1] On death, remove enemy from list, tell the spawner to spawn a new enemy, and destroy self
  (`ActorComponent.K2_DestroyComponent` (`self.HealthBar`))
  (`DestructibleComponent.ApplyRadiusDamage` (`self.DestructibleMesh`) 100.0 (`SceneComponent.K2_GetComponentLocation` (`self.CapsuleComponent`)) 100.0 100.0 true)
  (`KismetSystemLibrary.Delay` 2.0)
  (bind _asenemy_bp_spawner (cast `/Game/Enemy_BP_Spawner` (`self.Enemy_BP_Spawner`)))
  (set `/Game/Enemy_BP_Spawner.EnemyToRemoveFromList` self _asenemy_bp_spawner)
  (`/Game/Enemy_BP_Spawner.Event RemoveEnemyFromList` _asenemy_bp_spawner)
  (`/Game/Enemy_BP_Spawner.Event SpawnSingleEnemy` _asenemy_bp_spawner)
  (`self.K2_DestroyActor`))

(fn `UserConstructionScript`)